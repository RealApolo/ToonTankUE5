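; BP_TankPawn is the player-controlled tank pawn, wiring Enhanced Input to movement, rotation and firing.
; On BeginPlay, SetUpController casts the controller to PlayerController and adds the IMC_DefaultControls mapping context.
; Vertical and horizontal axis actions feed MoveVertical and Rotate, and the mouse action calls Fire.
; These three functions are not defined in this Blueprint, which only routes input to them.
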(event `self.ReceiveBeginPlay`
  (bind _asplayer_controller (cast `PlayerController` (`self.GetController`)))
  (message `EnhancedInputSubsystemInterface.AddMappingContext` (pcsubsystem `EnhancedInputLocalPlayerSubsystem` _asplayer_controller) "/Game/Inputs/IMC_DefaultControls.IMC_DefaultControls" 0 (struct)))

(event `EnhancedInput|/Game/Inputs/IA_VerticalAxis`
  (params (ActionValue :type "Float (double-precision)") (ElapsedSeconds :type "Float (double-precision)") (TriggeredSeconds :type "Float (double-precision)") (InputAction :type "InputAction Object Reference" :default "/Game/Inputs/IA_VerticalAxis.IA_VerticalAxis"))
  (:`Triggered`
    (`self.MoveVertical` ActionValue)))

(event `EnhancedInput|/Game/Inputs/IA_HorizontalAxis`
  (params (ActionValue :type "Float (double-precision)") (ElapsedSeconds :type "Float (double-precision)") (TriggeredSeconds :type "Float (double-precision)") (InputAction :type "InputAction Object Reference" :default "/Game/Inputs/IA_HorizontalAxis.IA_HorizontalAxis"))
  (:`Triggered`
    (`self.Rotate` ActionValue)))

(event `EnhancedInput|/Game/Inputs/IA_Mouse`
  (params (ActionValue :type Boolean) (ElapsedSeconds :type "Float (double-precision)") (TriggeredSeconds :type "Float (double-precision)") (InputAction :type "InputAction Object Reference" :default "/Game/Inputs/IA_Mouse.IA_Mouse"))
  (:`Triggered`
    (`self.Fire`)))

(fn `UserConstructionScript`)